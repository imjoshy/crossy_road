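; Police car actor that drives along its local forward axis and destroys itself after about 7000 units of travel, clearing CarExists.
; When LightOn is set, Tick restarts a timeline that updates the light color and swaps red and blue on finish.
; BeginPlay stops engine audio and spawns an attached siren, noted as not working.
; An audio play call and an alternating two-light flasher, noted for possible train warning lights, are left unconnected.
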(event EventBeginPlay
  ;[1 1 1] sounds
  ;;[1 1 1] engine noise
  (Audio|Components|Audio|Stop (Variables|Default|GetAudio))
  (if (Variables|Default|Getlight_on)
    ;;[1 1 1] siren -- DOESN'T WORK
    (Audio|SpawnSoundAttached "/Game/Assets/sounds/police/siren.siren" (Variables|Default|GetMediaSound) "None" "0, 0, 0" "0, 0, 0" "KeepRelativeOffset" true 1.0 1.0 0.0 "/Game/Assets/sounds/SoundAttenuation.SoundAttenuation" "/Game/Assets/sounds/SoundConcurrency.SoundConcurrency")))

(event EventTick
  (params (DeltaSeconds :type Float%20%28single-precision%29))
  (bind _forwardspeed (Variables|Default|GetforwardSpeed))
  (bind _multiplier (Variables|Default|Getmultiplier))
  (bind _returnvalue (* DeltaSeconds _forwardspeed))
  (bind _returnvalue_2 (* _returnvalue _multiplier))
  (Variables|Default|Setdistance_moved (+ (Variables|Default|Getdistance_moved) _returnvalue_2))
  (Transformation|AddActorLocalOffset (Math|Vector|MakeVector _returnvalue_2 0.0 0.0) false false)
  (if (Variables|Default|Getlight_on)
    ;[1 1 1] Wee woo wee woo
    (Timeline|Timeline_0 PlayFromStart
      (:Update
        (Rendering|Components|Light|SetLightColor (Variables|Default|Getwee_woo_wee_woo) (Utilities|Struct|MakeLinearColor (Math|Conversions|ToFloat(Integer) (Variables|Default|Getred_light)) 0.0 (Math|Conversions|ToFloat(Integer) (Variables|Default|Getblue_light)) 1.0) true)
        (if (>= (Math|Float|Absolute(Float) (Variables|Default|Getdistance_moved)) 7e+03) :!label _label
          (Actor|DestroyActor)
          (Variables|Default|Setcar_exists false)))
      (:Finished
        (if (== (Variables|Default|Getred_light) 0)
          (Variables|Default|Setred_light 255)
          (Variables|Default|Setblue_light 0)
          (else
            (Variables|Default|Setblue_light 255)
            (Variables|Default|Setred_light 0)))))
    (else
      (goto _label))))

(fn ConstructionScript)