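; A car actor that drives in a straight line and plays engine audio when the player comes near.
; Tick moves it along its local X axis by speed and multiplier, destroying it and clearing CarExists once the accumulated distance reaches a fixed limit.
; Engine, also called each Tick, starts the audio once when the player character is within a world-space X/Y range, latched by Playing.
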(event EventBeginPlay
  (Audio|Components|Audio|Stop (Variables|Default|GetAudio)))

(event EventTick
  (params (DeltaSeconds :type Float%20%28single-precision%29))
  (bind _forwardspeed (Variables|Default|GetforwardSpeed))
  (bind _multiplier (Variables|Default|Getmultiplier))
  (bind _returnvalue (* DeltaSeconds _forwardspeed))
  (bind _returnvalue_2 (* _returnvalue _multiplier))
  (Utilities|FlowControl|Sequence
    (:then_0
      (Variables|Default|Setdistance_moved (+ (Variables|Default|Getdistance_moved) _returnvalue_2))
      (Transformation|AddActorLocalOffset (Math|Vector|MakeVector _returnvalue_2 0.0 0.0) false false)
      (if (>= (Math|Float|Absolute(Float) (Variables|Default|Getdistance_moved)) 7e+03)
        (Actor|DestroyActor)
        (Variables|Default|Setcar_exists false)))
    (:then_1
      (CallFunction|Engine))))

(fn ConstructionScript)

(fn Engine
  (bind _returnvalue (Game|GetPlayerCharacter 0))
  (bind _returnvalue_2 (Transformation|GetActorLocation))
  (bind _returnvalue_3 (Transformation|GetActorLocation _returnvalue))
  (if (and (not (Variables|Default|Getplaying)) (and (<= (Math|Float|Absolute(Float) (- (.x _returnvalue_3) (.x _returnvalue_2))) 5e+02) (<= (Math|Float|Absolute(Float) (- (.y _returnvalue_3) (.y _returnvalue_2))) 1e+03)))
    (Audio|Components|Audio|Play (Variables|Default|GetAudio) 0.0)
    (Variables|Default|Setplaying true)))