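; Lane spawner that builds a crossing-style level forward along X, starting with one grass lane and four random lanes at BeginPlay.
; Each SpawnLane picks road, grass or railroad, passes the spawned lane a reference to this spawner, adds side barriers and advances the X cursor.
; Roads get two vehicle spawners and railroads one train spawner, each randomly left or right.
; SpawnRiver is an empty stub.
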(event EventBeginPlay
  (CallFunction|SpawnInitialLane)
  (CallFunction|SpawnLane)
  (CallFunction|SpawnLane)
  (CallFunction|SpawnLane)
  (CallFunction|SpawnLane))

(event Collision|EventActorBeginOverlap
  (params (OtherActor :type Actor%20Object%20Reference)))

(event EventTick
  (params (DeltaSeconds :type Float%20%28single-precision%29)))

(fn ConstructionScript)

(fn SpawnInitialLane
  ;[1 1 1] will always be grass
  (CallFunction|SpawnGrass))

(fn SpawnRoad
  ;[1 1 1] spawn road + vehicle spawners
  (bind _returnvalue (Game|SpawnActorfromClass "/Game/Blueprints/BP_road.BP_road_C" (Math|Transform|MakeTransform (Math|Vector|MakeVector (Variables|Default|Getspawn_loc_x) -5.9e+02 (Variables|Default|Getroad_z)) "0, 0, 0" "1,1,1") "Undefined" 0 0))
  (Variables|/Game/Blueprints/BP_road.BP_road_C|Setroad_spawner_ref _returnvalue self)
  (CallFunction|SpawnBarriers)
  (Utilities|FlowControl|Sequence ; Vehicle spawners on road lane
    (:then_0
      ;;[1 1 1] First lane -- road spawn loc - 75
      (Variables|Default|Setvehicle_spawn_loc_x (- (Variables|Default|Getspawn_loc_x) 75.0))
      (CallFunction|SpawnVehicle))
    (:then_1
      ;;[1 1 1] Second lane -- 70 ahead of first lane
      (Variables|Default|Setvehicle_spawn_loc_x (+ (Variables|Default|Getvehicle_spawn_loc_x) 7e+01))
      (CallFunction|SpawnVehicle)
      (Variables|Default|Setspawn_loc_x (+ (Variables|Default|Getspawn_loc_x) 1.6e+02)))))

(fn SpawnVehicle
  (if (== (Math|Random|RandomIntegerinRange 0 1) 0)
    (CallFunction|SpawnVehicleLeft)
    (else
      (CallFunction|SpawnVehicleRight))))

(fn SpawnVehicleLeft
  (Game|SpawnActorfromClass "/Game/Blueprints/vehicle_spawner_LEFT.vehicle_spawner_LEFT_C" (Math|Transform|MakeTransform (Math|Vector|MakeVector (Variables|Default|Getvehicle_spawn_loc_x) -7e+02 0.0) "0, 0, 0" "1,1,1") "Undefined" 0 0))

(fn SpawnVehicleRight
  (Game|SpawnActorfromClass "/Game/Blueprints/vehicle_spawner_RIGHT.vehicle_spawner_RIGHT_C" (Math|Transform|MakeTransform (Math|Vector|MakeVector (Variables|Default|Getvehicle_spawn_loc_x) 7e+03 0.0) "0, 0, 0" "1,1,1") "Undefined" 0 0))

(fn SpawnBarriers
  ;[1 1 1] left barrier -- limit movement to the left
  (Game|SpawnActorfromClass "/Game/Blueprints/barrier.barrier_C" (Math|Transform|MakeTransform (Math|Vector|MakeVector (Variables|Default|Getspawn_loc_x) (Variables|Default|Getleft_most) 2e+01) "0, 0, 0" "1,1,1") "Undefined" 0 0)
  ;[1 1 1] right barrier -- limit movement to the right
  (Game|SpawnActorfromClass "/Game/Blueprints/barrier.barrier_C" (Math|Transform|MakeTransform (Math|Vector|MakeVector (Variables|Default|Getspawn_loc_x) (Variables|Default|Getright_most) 2e+01) "0, 0, 0" "1,1,1") "Undefined" 0 0))

(fn SpawnLane
  (bind _output_get (Variables|Default|Setspawn_num (Math|Random|RandomIntegerinRange 0 2)))
  (if (== _output_get 0)
    (CallFunction|SpawnRoad)
    (elif (== _output_get 1)
      (CallFunction|SpawnGrass)
      (elif (== _output_get 2)
        (CallFunction|SpawnRr)))))

(fn SpawnRr
  (bind _returnvalue (Game|SpawnActorfromClass "/Game/Blueprints/BP_railroad.BP_railroad_C" (Math|Transform|MakeTransform (Math|Vector|MakeVector (Variables|Default|Getspawn_loc_x) -5.9e+02 (Variables|Default|Getroad_z)) "0, 0, 0" "1,1,1") "Undefined" 0 0))
  (Variables|/Game/Blueprints/BP_railroad.BP_railroad_C|Setroad_spawner_ref _returnvalue self)
  (CallFunction|SpawnBarriers)
  (CallFunction|SpawnTrain)
  (Variables|Default|Setspawn_loc_x (+ (Variables|Default|Getspawn_loc_x) 1.6e+02)))

(fn SpawnRiver)

(fn SpawnGrass
  (bind _returnvalue (Game|SpawnActorfromClass "/Game/Blueprints/BP_grass.BP_grass_C" (Math|Transform|MakeTransform (Math|Vector|MakeVector (Variables|Default|Getspawn_loc_x) -5.9e+02 2e+01) "0, 0, 0" "1,1,1") "Undefined" 0 0))
  (Variables|/Game/Blueprints/BP_grass.BP_grass_C|Setroad_spawner_ref _returnvalue self)
  (CallFunction|SpawnBarriers)
  (Variables|Default|Setspawn_loc_x (+ (Variables|Default|Getspawn_loc_x) 1.6e+02)))

(fn SpawnTrain
  (if (== (Math|Random|RandomIntegerinRange 0 1) 0)
    (CallFunction|SpawnTrainLeft)
    (else
      (CallFunction|SpawnTrainRight))))

(fn SpawnTrainLeft
  (Game|SpawnActorfromClass "/Game/Blueprints/train_spawner_LEFT.train_spawner_LEFT_C" (Math|Transform|MakeTransform (Math|Vector|MakeVector (Variables|Default|Getspawn_loc_x) -7e+02 2e+01) "0, 0, 0" "1,1,1") "Undefined" 0 0))

(fn SpawnTrainRight
  (Game|SpawnActorfromClass "/Game/Blueprints/train_spawner_RIGHT.train_spawner_RIGHT_C" (Math|Transform|MakeTransform (Math|Vector|MakeVector (Variables|Default|Getspawn_loc_x) 7e+03 2e+01) "0, 0, 0" "1,1,1") "Undefined" 0 0))