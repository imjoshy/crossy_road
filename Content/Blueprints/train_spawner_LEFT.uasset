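; Left-side train spawner that periodically spawns newTrain_v2 actors near its own position, at a fixed height and rotation.
; BeginPlay picks a random negative Multiplier once, which is passed to every train it spawns.
; Tick acts as the spawn timer, re-randomizing its own interval to a few seconds on each firing.
; After each spawn, the spawner destroys itself if the player character is far enough ahead along X.
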(event EventBeginPlay
  (Actor|Tick|SetActorTickInterval (Utilities|Select :Index (Math|Random|RandomIntegerinRange 0 2) :Option%200 4.0 :Option%201 5.0 :Option%202 6.0))
  (Variables|Default|Setmult (Utilities|Select :Index (Math|Random|RandomIntegerinRange 0 3) :Option%200 -4 :Option%201 -5 :Option%202 -6 :Option%203 -7)))

(event Collision|EventActorBeginOverlap
  (params (OtherActor :type Actor%20Object%20Reference)))

(event EventTick
  (params (DeltaSeconds :type Float%20%28single-precision%29))
  (bind _returnvalue (Transformation|GetActorLocation))
  (Actor|Tick|SetActorTickInterval (Utilities|Select :Index (Math|Random|RandomIntegerinRange 0 2) :Option%200 4.0 :Option%201 5.0 :Option%202 6.0))
  (Utilities|FlowControl|Sequence
    (:then_0
      (bind _returnvalue_2 (Game|SpawnActorfromClass "/Game/Blueprints/train_v2.train_v2_C" (Math|Transform|MakeTransform (Math|Vector|MakeVector (+ (.x _returnvalue) 5e+01) (.y _returnvalue) -1.3e+02) "0.000000,270.000000,0.000000" "1.500000,1.500000,1.500000") "Undefined" 0 0))
      (Variables|/Game/Blueprints/train_v2.train_v2_C|Setmultiplier _returnvalue_2 (Math|Conversions|ToFloat(Integer) (Variables|Default|Getmult))))
    (:then_1
      (if (and (< (.x (Transformation|GetActorLocation)) (.x (Transformation|GetActorLocation (Game|GetPlayerCharacter 0)))) (> (- (Math|Float|Absolute(Float) (.x (Transformation|GetActorLocation (Game|GetPlayerCharacter 0)))) (Math|Float|Absolute(Float) (.x (Transformation|GetActorLocation)))) 5e+02))
        (Actor|DestroyActor)))))

(fn ConstructionScript)